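; Mummy enemy that detects the player by sight and is destroyed when its health runs out.
; A pawn sensing component sets the "hasSeenPlayer?" blackboard key on its AI controller when it sees a BP_TopDownCharacter; nothing here clears the key.
; Tick polls Health every frame and destroys the actor at zero or below.
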(event OnSeePawn(PawnSensing_Mummy)
  (params (Pawn :type Pawn%20Object%20Reference))
  (Utilities|Casting|CastToBP_TopDownCharacter Pawn)
  (AI|Components|Blackboard|SetValueasBool (AI|GetBlackboard (AI|GetAIController self)) (Utilities|Name|MakeLiteralName "hasSeenPlayer?") true))

(event EventBeginPlay)

(event Collision|EventActorBeginOverlap
  (params (OtherActor :type Actor%20Object%20Reference)))

(event EventTick
  (params (DeltaSeconds :type Float%20%28single-precision%29))
  (if (<= (Variables|Default|GetHealth) 0)
    (Actor|DestroyActor)))

(fn ConstructionScript)